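; Cannon actor that repeatedly launches Bp_projectileroller projectiles from its Arrow component.
; BeginPlay stores the mesh's starting rotation and starts a looping timer, presumably driving the Fire! event.
; Fire! spawns each projectile with launch speed and gravity scale randomized around LaunchPower and Weight, plus a set lifespan.
; After each spawn, it randomizes the mesh's yaw slightly around the stored rotation, avoiding cumulative drift.
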(event `self.ReceiveBeginPlay`
  (`KismetSystemLibrary.K2_SetTimerDelegate` (`|CreateDelegate` :!event `Fire!`) (`self.Time`) true)
  (set `self.Rotator` (`SceneComponent.K2_GetComponentRotation` (`self.StaticMesh`))))

(event `Fire!`
  (bind _weight (`self.Weight`))
  (bind _launch_power (`self.Launch Power`))
  (bind (_rotator_roll _rotator_pitch _rotator_yaw) (`KismetMathLibrary.BreakRotator` (`self.Rotator`)))
  (bind (_returnvalue_location _returnvalue_rotation) (`KismetMathLibrary.BreakTransform` (`SceneComponent.K2_GetComponentToWorld` (`self.Arrow`))))
  (`|SpawnActorFromClass` "/Game/Tech/Harvey/BluePrints/Projectiles/bp_projectileroller.bp_projectileroller_C" (`KismetMathLibrary.MakeTransform` _returnvalue_location _returnvalue_rotation (`self.Spawn Transform Scale`)) "Undefined" "OverrideRootScale" null (`KismetMathLibrary.RandomFloatInRange` (- _weight 0.1) (+ _weight 0.1)) (`KismetMathLibrary.RandomFloatInRange` (- _launch_power 50.0) (+ _launch_power 50.0)) (`self.Life Span`) null)
  (`SceneComponent.K2_SetWorldRotation` (`self.StaticMesh`) (`KismetMathLibrary.MakeRotator` _rotator_roll _rotator_pitch (`KismetMathLibrary.RandomFloatInRange` (- _rotator_yaw 7.5) (+ _rotator_yaw 7.5))) false false))

(fn `UserConstructionScript`)