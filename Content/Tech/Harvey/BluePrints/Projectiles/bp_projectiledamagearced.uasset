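; Arced damage projectile Blueprint that knocks the main character into ragdoll on contact.
; On BeginPlay it copies its gravity scale and speed variables into ProjectileMovement, setting max speed equal to initial speed.
; A collision overlap with BP_MainCharacter either takes a hit off the shield if the character is immune or triggers ragdoll, then destroys the projectile.
; A mesh hit also destroys it.
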(event `self.ReceiveBeginPlay`
  (bind _projectilemovement (`self.ProjectileMovement`))
  ;[1 1 1] If you want to change the gravity of the projectile
  (set `ProjectileMovementComponent.ProjectileGravityScale` (`self.Projectile Gravity Scale`) _projectilemovement)
  (bind _output_get (set `ProjectileMovementComponent.InitialSpeed` (`self.Speed`) _projectilemovement))
  (set `ProjectileMovementComponent.MaxSpeed` _output_get _projectilemovement))

(event `self.Collision.OnComponentBeginOverlap`
  (params (OverlappedComponent :type "PrimitiveComponent Object Reference") (OtherActor :type "Actor Object Reference") (OtherComp :type "PrimitiveComponent Object Reference") (OtherBodyIndex :type Integer) (bFromSweep :type Boolean) (SweepResult :type "HitResult Structure (by ref)"))
  ;[1 1 1] When the projectile hits a pawn
  (bind _asbp_main_character (cast `/Game/Tech/Cam/BP_MainCharacter` OtherActor))
  (if (`/Game/Tech/Cam/BP_MainCharacter.isImmune` _asbp_main_character)
    (`/Game/Tech/Cam/BP_MainCharacter.TakeHitOffShield` _asbp_main_character)
    (`self.K2_DestroyActor`)
    (else
      (`/Game/Tech/Cam/BP_MainCharacter.TriggerRagdoll` _asbp_main_character)
      (`self.K2_DestroyActor`))))

(event `self.ProjectileMesh.OnComponentHit`
  (params (HitComponent :type "PrimitiveComponent Object Reference") (OtherActor :type "Actor Object Reference") (OtherComp :type "PrimitiveComponent Object Reference") (NormalImpulse :type "Vector Structure") (Hit :type "HitResult Structure (by ref)"))
  ;[1 1 1] When the Projectile Hits something other than the Pawn
  (`self.K2_DestroyActor`))

(fn `UserConstructionScript`)