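; Rolling projectile Blueprint that destroys itself when its Roller component hits the main character, with a debug print standing in for a ragdoll effect.
; On other hits, it destroys both actors only if the other is the single roller that GetActorOfClass returns, so not every roller-to-roller collision matches.
; The construction script applies configurable gravity scale and initial speed to ProjectileMovement and sets the lifespan.
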(event `self.Roller.OnComponentHit`
  (params (HitComponent :type "PrimitiveComponent Object Reference") (OtherActor :type "Actor Object Reference") (OtherComp :type "PrimitiveComponent Object Reference") (NormalImpulse :type "Vector Structure") (Hit :type "HitResult Structure (by ref)"))
  (cast `/Game/Tech/Cam/BP_MainCharacter` OtherActor
    (:`then`
      (`KismetSystemLibrary.PrintString` "Add Ragdoll Plz")
      (`self.K2_DestroyActor`))
    (:`CastFailed`
      (bind _returnvalue (`GameplayStatics.GetActorOfClass` "bp_projectileroller_C"))
      (if (== OtherActor _returnvalue)
        (`self.K2_DestroyActor` OtherActor)
        (`self.K2_DestroyActor`)
        (`KismetSystemLibrary.PrintString` "Hello")))))

(fn `UserConstructionScript`
  (bind _projectilemovement (`self.ProjectileMovement`))
  (set `ProjectileMovementComponent.ProjectileGravityScale` (`self.Projectile Gravity Scale`) _projectilemovement)
  (set `ProjectileMovementComponent.InitialSpeed` (`self.Initial Speed`) _projectilemovement)
  (`self.SetLifeSpan` (`self.InitialLifeSpan`)))