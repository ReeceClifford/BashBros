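; Floor trap Blueprint that deals damage over time to actors inside its Box collision.
; Overlapping actors join ActorsInField, and each entry starts a looping timer that applies Damage to every listed actor at IntervalBetweenDamage.
; Exit removes the actor and clears DOTTimer, a single handle overwritten on each entry, so only the most recently started timer stops, even if others remain inside.
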(event `self.Box.OnComponentBeginOverlap`
  (params (OverlappedComponent :type "PrimitiveComponent Object Reference") (OtherActor :type "Actor Object Reference") (OtherComp :type "PrimitiveComponent Object Reference") (OtherBodyIndex :type Integer) (bFromSweep :type Boolean) (SweepResult :type "HitResult Structure (by ref)"))
  ;[1 1 1] When a Character Enters the collion box
  (`KismetArrayLibrary.Array_Add` (`self.ActorsInField`) OtherActor)
  (bind _returnvalue (`KismetSystemLibrary.K2_SetTimerDelegate` (delegate `StayTooLong`) (`self.IntervalBetweenDamage`) true))
  (set `self.DOTTimer` _returnvalue))

(event `StayTooLong`
  ;[1 1 1] When a Character Enters the collion box
  (for _array_element (`self.ActorsInField`)
    (`GameplayStatics.ApplyDamage` _array_element (`self.Damage`))))

(event `self.Box.OnComponentEndOverlap`
  (params (OverlappedComponent :type "PrimitiveComponent Object Reference") (OtherActor :type "Actor Object Reference") (OtherComp :type "PrimitiveComponent Object Reference") (OtherBodyIndex :type Integer))
  ;[1 1 1] When a character leaves the area
  (`KismetSystemLibrary.K2_ClearAndInvalidateTimerHandle` (`self.DOTTimer`))
  (`KismetArrayLibrary.Array_RemoveItem` (`self.ActorsInField`) OtherActor))

(fn `UserConstructionScript`)