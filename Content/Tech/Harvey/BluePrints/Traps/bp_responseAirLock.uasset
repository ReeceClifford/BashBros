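; Airlock trap response that, when triggered, opens a door and drags overlapping actors out along an arrow's direction.
; A timeline lerps the door between closed and opened positions, reversing on untrigger, and its alpha also scales suction strength.
; A looping timer set on BeginPlay appears to drive the pull on actors tracked by the suction volume.
; The ConfirmKill overlap only prints a kill message.
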(event `self.ReceiveBeginPlay`
  ;[1 1 1] Set up the pulling motion and the door opening
  (set `self.Closed Position` (`SceneComponent.RelativeLocation` (`self.Door`)))
  (set `self.OpenedPosition` (`SceneComponent.RelativeLocation` (`self.OpenedDoor`)))
  (`KismetSystemLibrary.K2_SetTimerDelegate` (`|CreateDelegate` :!event `SuckedOut`) 0.01 true)
  (`TimelineComponent.SetPlayRate` (`self.Opening`) (`self.DoorOpeningSpeed`)))

(event `/Game/Tech/Harvey/BluePrints/Interface/bpint_LockAndKey.Trigger`
  ;[1 1 1] Open the Door
  (bind (_direction _dooropening) (`Timeline|Opening` :!label _label)
    (:`Update`
      (`SceneComponent.K2_SetRelativeLocation` (`self.Door`) (`KismetMathLibrary.VLerp` (`self.Closed Position`) (`self.OpenedPosition`) _dooropening) false false))))

(event `/Game/Tech/Harvey/BluePrints/Interface/bpint_LockAndKey.UnTrigger`
  ;[1 1 1] Open the Door
  (goto _label :!via `Reverse`))

(event `self.Volume.OnComponentBeginOverlap`
  (params (OverlappedComponent :type "PrimitiveComponent Object Reference") (OtherActor :type "Actor Object Reference") (OtherComp :type "PrimitiveComponent Object Reference") (OtherBodyIndex :type Integer) (bFromSweep :type Boolean) (SweepResult :type "HitResult Structure (by ref)"))
  ;[1 1 1] Getting Sucked Out of the Airlock
  (`KismetArrayLibrary.Array_Add` (`self.ActorsSuckedOut`) OtherActor))

(event `SuckedOut`
  ;[1 1 1] Getting Sucked Out of the Airlock
  (for _array_element (`self.ActorsSuckedOut`)
    (`self.K2_AddActorWorldOffset` _array_element (* (`SceneComponent.GetForwardVector` (`self.Arrow`)) (stale `/Game/Tech/Harvey/BluePrints/Interface/bpint_LockAndKey.Trigger` _dooropening) (`self.SuctionSpeed`)) false false)))

(event `self.Volume.OnComponentEndOverlap`
  (params (OverlappedComponent :type "PrimitiveComponent Object Reference") (OtherActor :type "Actor Object Reference") (OtherComp :type "PrimitiveComponent Object Reference") (OtherBodyIndex :type Integer))
  ;[1 1 1] Getting Sucked Out of the Airlock
  (`KismetArrayLibrary.Array_RemoveItem` (`self.ActorsSuckedOut`) OtherActor))

(event `self.ConfirmKill.OnComponentBeginOverlap`
  (params (OverlappedComponent :type "PrimitiveComponent Object Reference") (OtherActor :type "Actor Object Reference") (OtherComp :type "PrimitiveComponent Object Reference") (OtherBodyIndex :type Integer) (bFromSweep :type Boolean) (SweepResult :type "HitResult Structure (by ref)"))
  ;[1 1 1] When they are fully out the door
  (`KismetSystemLibrary.PrintString` (`KismetTextLibrary.Conv_TextToString` (`|FormatText` "Kill {Actor}" OtherActor))))

(fn `UserConstructionScript`
  (`parent.UserConstructionScript`))