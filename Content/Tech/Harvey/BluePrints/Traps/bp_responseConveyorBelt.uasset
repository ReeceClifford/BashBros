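; Trap response conveyor belt that pushes actors inside its collision box along the direction of an Arrow component.
; Box overlaps maintain the list of affected actors, and a fast looping timer offsets each one without sweep, scaled by Speed.
; Trigger from a connected trap negates the Arrow's starting world rotation to reverse the belt, and UnTrigger restores it.
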(event `self.ReceiveBeginPlay`
  ;[1 1 1] Timer which pushes every character in the conveyor
  (`KismetSystemLibrary.K2_SetTimerDelegate` (delegate `PushFromConveyor`) 0.01 true)
  (set `self.OriginRotation` (`SceneComponent.K2_GetComponentRotation` (`self.Arrow`))))

(event `PushFromConveyor`
  ;[1 1 1] Timer which pushes every character in the conveyor
  (for _array_element (`self.inConveyor`)
    (`self.K2_AddActorWorldOffset` _array_element (* (`SceneComponent.GetForwardVector` (`self.Arrow`)) (`self.Speed`)) false false)))

(event `self.Box.OnComponentBeginOverlap`
  (params (OverlappedComponent :type "PrimitiveComponent Object Reference") (OtherActor :type "Actor Object Reference") (OtherComp :type "PrimitiveComponent Object Reference") (OtherBodyIndex :type Integer) (bFromSweep :type Boolean) (SweepResult :type "HitResult Structure (by ref)"))
  ;[1 1 1] When an actor moves into the collision box add them to the queue
  (`KismetArrayLibrary.Array_Add` (`self.inConveyor`) OtherActor))

(event `self.Box.OnComponentEndOverlap`
  (params (OverlappedComponent :type "PrimitiveComponent Object Reference") (OtherActor :type "Actor Object Reference") (OtherComp :type "PrimitiveComponent Object Reference") (OtherBodyIndex :type Integer))
  ;[1 1 1] When they leave, remove them from the list so they won't experience any other forces
  (`KismetArrayLibrary.Array_RemoveItem` (`self.inConveyor`) OtherActor))

(event `/Game/Tech/Harvey/BluePrints/Interface/bpint_LockAndKey.Trigger`
  ;[1 1 1] When a trap connected to this is activated, reverse the arrow, the asset controlling the direction of the conveyor
  (`SceneComponent.K2_SetWorldRotation` (`self.Arrow`) (* (`self.OriginRotation`) -1.0) false false))

(event `/Game/Tech/Harvey/BluePrints/Interface/bpint_LockAndKey.UnTrigger`
  ;[1 1 1] Resets if the trigger can be repeated
  (`SceneComponent.K2_SetWorldRotation` (`self.Arrow`) (`self.OriginRotation`) false false))

(fn `UserConstructionScript`
  (`parent.UserConstructionScript`))