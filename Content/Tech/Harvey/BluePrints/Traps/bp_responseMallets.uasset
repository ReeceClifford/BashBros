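; Mallet trap that swings when triggered and ragdolls the main character on contact, or takes a hit off the shield if the character is immune.
; BeginPlay caches the root's start rotation and the Prediciton component's rotation as the end pose, then calls CheckIfInfinite.
; Trigger restarts the Slam timeline, whose Rotation track feeds RInterpTo's DeltaTime as a blend between those rotations.
; Box overlap handles the hit independently of the swing.
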(event `self.ReceiveBeginPlay`
  ;[1 1 1] Set Rotators and Infinite Loops
  (set `self.Origin` (`SceneComponent.K2_GetComponentRotation` (`self.DefaultSceneRoot`)))
  (set `self.End` (`SceneComponent.K2_GetComponentRotation` (`self.Prediciton`)))
  (`self.CheckIfInfinite`))

(event `/Game/Tech/Harvey/BluePrints/Interface/bpint_LockAndKey.Trigger`
  ;[1 1 1] Trap
  (bind (_direction _rotation) (`Timeline|Slam` :!via `PlayFromStart`)
    (:`Update`
      (`SceneComponent.K2_SetWorldRotation` (`self.DefaultSceneRoot`) (`KismetMathLibrary.RInterpTo` (`self.Origin`) (`self.End`) _rotation 1.0) false false))))

(event `self.Box.OnComponentBeginOverlap`
  (params (OverlappedComponent :type "PrimitiveComponent Object Reference") (OtherActor :type "Actor Object Reference") (OtherComp :type "PrimitiveComponent Object Reference") (OtherBodyIndex :type Integer) (bFromSweep :type Boolean) (SweepResult :type "HitResult Structure (by ref)"))
  ;[1 1 1] Trap
  (bind _asbp_main_character (cast `/Game/Tech/Cam/BP_MainCharacter` OtherActor))
  (if (`/Game/Tech/Cam/BP_MainCharacter.isImmune` _asbp_main_character)
    (`/Game/Tech/Cam/BP_MainCharacter.TakeHitOffShield` _asbp_main_character)
    (else
      (`/Game/Tech/Cam/BP_MainCharacter.TriggerRagdoll` _asbp_main_character))))

(fn `UserConstructionScript`
  (`parent.UserConstructionScript`))