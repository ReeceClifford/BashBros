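; Trap response actor that, when triggered, moves a pushing object toward a destination component and damages actors that touch its box.
; BeginPlay caches both world transforms and sets the Movement timeline's play rate.
; Trigger plays that timeline to lerp the object between them without sweeping, then rewinds the timeline time on finish for reuse.
; Box overlaps apply damage to any actor and print the damage result.
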(event `self.ReceiveBeginPlay`
  ;[1 1 1] Set up the origin and destination and play speed
  (set `self.OriginLocation` (`SceneComponent.K2_GetComponentToWorld` (`self.PushingObject`)))
  (set `self.DestinationLocation` (`SceneComponent.K2_GetComponentToWorld` (`self.Destination`)))
  (`TimelineComponent.SetPlayRate` (`self.Movement`) (`self.Movement Rate`)))

(event `/Game/Tech/Harvey/BluePrints/Interface/bpint_LockAndKey.Trigger`
  ;[1 1 1] Goes to where the destination mesh is in the world
  (bind (_direction _movetoend) (`Timeline|Movement`)
    (:`Update`
      (`SceneComponent.K2_SetWorldTransform` (`self.PushingObject`) (`KismetMathLibrary.TLerp` (`self.OriginLocation`) (`self.DestinationLocation`) _movetoend) false false))
    (:`Finished`
      ;[1 1 1] Timeline Resets when it finishes its movement
      (`TimelineComponent.SetNewTime` (`self.Movement`) 0.0))))

(event `self.Box.OnComponentBeginOverlap`
  (params (OverlappedComponent :type "PrimitiveComponent Object Reference") (OtherActor :type "Actor Object Reference") (OtherComp :type "PrimitiveComponent Object Reference") (OtherBodyIndex :type Integer) (bFromSweep :type Boolean) (SweepResult :type "HitResult Structure (by ref)"))
  ;[1 1 1] If any pawn overlaps the collision, they take damage
  (bind _returnvalue (`GameplayStatics.ApplyDamage` OtherActor (`self.Damage`)))
  (`KismetSystemLibrary.PrintString` (`KismetStringLibrary.Conv_DoubleToString` _returnvalue)))

(fn `UserConstructionScript`
  (`parent.UserConstructionScript`))