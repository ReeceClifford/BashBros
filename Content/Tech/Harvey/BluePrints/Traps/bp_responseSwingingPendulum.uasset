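; Swinging pendulum trap that damages actors overlapping its box and ragdolls the main character on contact.
; On BeginPlay it stores the root's transform, builds a destination with a new rotation, sets the timeline play rate and calls CheckIfInfinite.
; Trigger plays the Movement timeline, which lerps the root to the destination using Euler interpolation, then reverses it back to the origin.
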(event `self.ReceiveBeginPlay`
  (bind (_returnvalue_location _returnvalue_rotation _returnvalue_scale) (`KismetMathLibrary.BreakTransform` (`SceneComponent.K2_GetComponentToWorld` (`self.DefaultSceneRoot`))))
  ;[1 1 1] Set up the original rotation
  (set `self.OriginLocation` (`KismetMathLibrary.MakeTransform` _returnvalue_location _returnvalue_rotation _returnvalue_scale))
  (set `self.Destination` (`KismetMathLibrary.MakeTransform` _returnvalue_location (`self.RotationToDestination`) _returnvalue_scale))
  (`TimelineComponent.SetPlayRate` (`self.Movement`) (`self.Play Rate`))
  (`self.CheckIfInfinite`))

(event `/Game/Tech/Harvey/BluePrints/Interface/bpint_LockAndKey.Trigger`
  ;[1 1 1] Rotates the pendulum
  (bind (_direction _movetoend) (`Timeline|Movement` :!label _label)
    (:`Update`
      (`SceneComponent.K2_SetWorldTransform` (`self.DefaultSceneRoot`) (`KismetMathLibrary.TLerp` (`self.OriginLocation`) (`self.Destination`) _movetoend "EulerInterp") false false))
    (:`Finished`
      (if (`|EnumEquality` _direction "Forward")
        (goto _label :!via `Reverse`)))))

(event `self.Box.OnComponentBeginOverlap`
  (params (OverlappedComponent :type "PrimitiveComponent Object Reference") (OtherActor :type "Actor Object Reference") (OtherComp :type "PrimitiveComponent Object Reference") (OtherBodyIndex :type Integer) (bFromSweep :type Boolean) (SweepResult :type "HitResult Structure (by ref)"))
  ;[1 1 1] if any pawn hits the pendulum.
  (`GameplayStatics.ApplyDamage` OtherActor (`self.Damage`))
  (bind _asbp_main_character (cast `/Game/Tech/Cam/BP_MainCharacter` OtherActor))
  (`/Game/Tech/Cam/BP_MainCharacter.TriggerRagdoll` _asbp_main_character))

(fn `UserConstructionScript`
  (`parent.UserConstructionScript`))