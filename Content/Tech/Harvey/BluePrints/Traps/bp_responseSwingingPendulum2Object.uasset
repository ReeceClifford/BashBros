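; A trap response actor: a pendulum that swings between its starting transform and that of a referenced Destination actor.
; On BeginPlay it stores both transforms, sets the timeline's play rate and calls CheckIfInfinite.
; Trigger plays the timeline, which lerps the root's transform to the destination and then reverses back.
; Its box overlap applies damage to the other actor and triggers ragdoll on BP_MainCharacter.
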(event `self.ReceiveBeginPlay`
  ;[1 1 1] Set up the original rotation
  (set `self.OriginLocation` (`SceneComponent.K2_GetComponentToWorld` (`self.DefaultSceneRoot`)))
  (set `self.DestinationTrans` (`SceneComponent.K2_GetComponentToWorld` (`Actor.RootComponent` (`self.Destination`))))
  (`TimelineComponent.SetPlayRate` (`self.Movement`) (`self.Play Rate`))
  (`self.CheckIfInfinite`))

(event `/Game/Tech/Harvey/BluePrints/Interface/bpint_LockAndKey.Trigger`
  ;[1 1 1] Rotates the pendulum
  (bind (_direction _movetoend) (`Timeline|Movement` :!label _label)
    (:`Update`
      (`SceneComponent.K2_SetWorldTransform` (`self.DefaultSceneRoot`) (`KismetMathLibrary.TLerp` (`self.OriginLocation`) (`self.DestinationTrans`) _movetoend) false false))
    (:`Finished`
      (if (`|EnumEquality` _direction "Forward")
        (goto _label :!via `Reverse`)))))

(event `self.Box.OnComponentBeginOverlap`
  (params (OverlappedComponent :type "PrimitiveComponent Object Reference") (OtherActor :type "Actor Object Reference") (OtherComp :type "PrimitiveComponent Object Reference") (OtherBodyIndex :type Integer) (bFromSweep :type Boolean) (SweepResult :type "HitResult Structure (by ref)"))
  ;[1 1 1] if any pawn hits the pendulum.
  (`GameplayStatics.ApplyDamage` OtherActor (`self.Damage`))
  (bind _asbp_main_character (cast `/Game/Tech/Cam/BP_MainCharacter` OtherActor))
  (`/Game/Tech/Cam/BP_MainCharacter.TriggerRagdoll` _asbp_main_character))

(fn `UserConstructionScript`
  (`parent.UserConstructionScript`))