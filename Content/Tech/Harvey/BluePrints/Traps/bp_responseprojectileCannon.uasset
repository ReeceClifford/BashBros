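; A triggered cannon trap that fires a damaging projectile after a configurable delay.
; Trigger starts the fire timer alongside a timeline that tints the mesh from near-white to red as a warning, then resets it to white.
; ProjectileSpawn creates a Bp_projectiledamagearcs at the arrow component's location and rotation, passing in scale, damage, speed and gravity scale.
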(event `/Game/Tech/Harvey/BluePrints/Interface/bpint_LockAndKey.Trigger`
  (bind _mesh (`self.Mesh`))
  ;[1 1 1] Triggers tell the cannon to shoot
  (`KismetSystemLibrary.K2_SetTimerDelegate` (`|CreateDelegate` :!event `ProjectileSpawn`) (`self.TimeTillFireing`))
  ;[1 1 1] This is to show when the cannon will fire
  (bind (_direction _firetime) (`Timeline|GoingToFire`)
    (:`Update`
      (`MeshComponent.SetVectorParameterValueOnMaterials` _mesh "Base Color" (`KismetMathLibrary.Conv_LinearColorToVector` (`KismetMathLibrary.LinearColorLerp` (struct :`R` 0.96706 :`G` 1.0 :`B` 0.989879 :`A` 1.0) (struct :`R` 1.0 :`A` 1.0) _firetime))))
    (:`Finished`
      (`MeshComponent.SetVectorParameterValueOnMaterials` _mesh "Base Color" (`KismetMathLibrary.Conv_LinearColorToVector` (`KismetMathLibrary.LinearColor_White`)))
      (`TimelineComponent.SetNewTime` (`self.GoingToFire`) 0.0))))

(event `ProjectileSpawn`
  (bind _projectilescale (`self.ProjectileScale`))
  (bind (_returnvalue_location _returnvalue_rotation) (`KismetMathLibrary.BreakTransform` (`SceneComponent.K2_GetComponentToWorld` (`self.Arrow`))))
  ;[1 1 1] Spawn Projectile when activated
  (`|SpawnActorFromClass` "/Game/Tech/Harvey/BluePrints/Projectiles/bp_projectiledamagearcs.bp_projectiledamagearcs_C" (`KismetMathLibrary.MakeTransform` _returnvalue_location _returnvalue_rotation (`KismetMathLibrary.MakeVector` _projectilescale _projectilescale _projectilescale)) "Undefined" "OverrideRootScale" null (`self.ProjectileDamage`) (`self.ProjectileGravityScale`) (`self.Speed`) null))

(fn `UserConstructionScript`
  (`parent.UserConstructionScript`))