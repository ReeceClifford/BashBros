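; Trapdoor response actor that swings open on Trigger and closes on UnTrigger.
; BeginPlay stores the Door component's world rotation, and Open plays or reverses the TrapdoorMovement timeline.
; Each update rotates the whole actor, not just Door, from that origin toward the origin minus DisplacementRotation, feeding the timeline value into RInterpToConstant as delta time.
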(event `/Game/Tech/Harvey/BluePrints/Interface/bpint_LockAndKey.Trigger`
  (`self.Open` true))

(event `self.ReceiveBeginPlay`
  (set `self.OriginRotation` (`SceneComponent.K2_GetComponentRotation` (`self.Door`))))

(event `/Game/Tech/Harvey/BluePrints/Interface/bpint_LockAndKey.UnTrigger`
  (`self.Open` false))

(event `Open`
  (params (`Open?` :type Boolean))
  (bind _originrotation (`self.OriginRotation`))
  (if `Open?`
    (bind (_direction _movement) (`Timeline|TrapdoorMovement` :!label _label)
      (:`Update`
        (`self.K2_SetActorRotation` (`KismetMathLibrary.RInterpTo_Constant` _originrotation (`KismetMathLibrary.NormalizedDeltaRotator` _originrotation (`self.DisplacementRotation`)) _movement 250.0))))
    (else
      (goto _label :!via `Reverse`))))

(fn `UserConstructionScript`
  (`parent.UserConstructionScript`))