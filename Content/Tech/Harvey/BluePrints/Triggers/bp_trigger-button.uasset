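; Pressure button trigger that fires the Trigger event on every trap in its TrapsToTrigger array when something overlaps its collider.
; A timeline lerps the button mesh down from its starting location, while PressingAction swaps its material to green.
; With Repeatable set, ending the overlap reverses the timeline and restores red; otherwise a DoOnce gates activation and the button stays pressed.
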(event `self.ReceiveBeginPlay`
  (set `self.OriginLocation` (`SceneComponent.RelativeLocation` (`self.Button`))))

(event `Pressed`
  (params (`True?` :type Boolean))
  (bind _originlocation (`self.OriginLocation`))
  (`self.PressingAction` `True?`)
  (if `True?`
    (bind (_direction _pressingmovement) (`Timeline|ButtonMovement` :!label _label)
      (:`Update`
        (`SceneComponent.K2_SetRelativeLocation` (`self.Button`) (`KismetMathLibrary.VLerp` _originlocation (- _originlocation (0.0 0.0 75.0)) _pressingmovement) false false)))
    (else
      (goto _label :!via `Reverse`))))

(event `self.ColliderForButton.OnComponentBeginOverlap`
  (params (OverlappedComponent :type "PrimitiveComponent Object Reference") (OtherActor :type "Actor Object Reference") (OtherComp :type "PrimitiveComponent Object Reference") (OtherBodyIndex :type Integer) (bFromSweep :type Boolean) (SweepResult :type "HitResult Structure (by ref)"))
  (if (not (`self.Repeatable?`))
    (`/Engine/EditorBlueprintResources/StandardMacros.DoOnce` false
      (:`Completed`
        _)))
  (for _array_element (`self.TrapsToTrigger`)
    (`/Game/Tech/Harvey/BluePrints/Interface/bpint_LockAndKey.Trigger` _array_element))
  (`self.Pressed` true))

(event `self.ColliderForButton.OnComponentEndOverlap`
  (params (OverlappedComponent :type "PrimitiveComponent Object Reference") (OtherActor :type "Actor Object Reference") (OtherComp :type "PrimitiveComponent Object Reference") (OtherBodyIndex :type Integer))
  (if (`self.Repeatable?`)
    (`self.Pressed` false)))

(fn `PressingAction`
  (params (`On?` :type Boolean))
  (bind _button (`self.Button`))
  (if `On?`
    (`PrimitiveComponent.SetMaterial` _button 0 "/Game/Tech/Harvey/Materials/MI_Solid_GreenDJ.MI_Solid_GreenDJ")
    (elif (`self.Repeatable?`)
      (`PrimitiveComponent.SetMaterial` _button 0 "/Game/Tech/Harvey/Materials/MI_Solid_RedDJ.MI_Solid_RedDJ"))))

(fn `UserConstructionScript`
  (`parent.UserConstructionScript`))