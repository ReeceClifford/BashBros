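; A trigger Blueprint that has a random chance to switch on a set of linked traps when something overlaps its collision component.
; Each overlap rolls a weighted random bool, and a success calls TriggerTraps to turn the assigned traps on, with no filter on the overlapping actor.
; A resetting trigger turns the traps off after a configurable delay, while a non-resetting one destroys itself right after firing.
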(event `self.Collision.OnComponentBeginOverlap`
  (params (OverlappedComponent :type "PrimitiveComponent Object Reference") (OtherActor :type "Actor Object Reference") (OtherComp :type "PrimitiveComponent Object Reference") (OtherBodyIndex :type Integer) (bFromSweep :type Boolean) (SweepResult :type "HitResult Structure (by ref)"))
  (bind _trapstotrigger (`self.TrapsToTrigger`))
  (if (`KismetMathLibrary.RandomBoolWithWeight` (`self.ChaceToTrigger`))
    (`self.TriggerTraps` _trapstotrigger true)
    (if (`self.Resets?`)
      (`KismetSystemLibrary.Delay` (`self.TimeTilReset`))
      (`self.TriggerTraps` _trapstotrigger)
      (else
        (`self.K2_DestroyActor`)))))

(fn `UserConstructionScript`
  (`parent.UserConstructionScript`))