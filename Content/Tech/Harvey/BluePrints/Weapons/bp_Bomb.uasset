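; Fused bomb weapon that knocks a BP_MainCharacter away when it explodes, with no damage applied.
; The construction script starts a looping fuse timer and sets a lifespan just past the fuse time.
; BANG! runs a debug-drawn, single-hit sphere trace for pawns at the mesh, then launches the character along the hit normal.
; Push force maps from that normal's length, not from distance to the blast.
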(event `BANG!`
  (bind _returnvalue (`SceneComponent.K2_GetComponentLocation` (`self.Mesh`)))
  (bind _outhit (`KismetSystemLibrary.SphereTraceSingleForObjects` :`Start` _returnvalue :`End` _returnvalue :`Radius` (`self.ExplosionRadius`) :`ObjectTypes` (`|MakeArray` "ObjectTypeQuery3" :!type "EObjectTypeQuery Enum") :`DrawDebugType` "ForDuration" :`DrawTime` 2.0))
  (bind (_bblockinghit _binitialoverlap _time _distance _location _impactpoint _normal _impactnormal _physmat _hitactor) (`GameplayStatics.BreakHitResult` _outhit))
  (bind _asbp_main_character (cast `/Game/Tech/Cam/BP_MainCharacter` _hitactor))
  (`Character.LaunchCharacter` _asbp_main_character (* _normal (`KismetMathLibrary.MapRangeClamped` (`KismetMathLibrary.VSize` _normal) 0.0 (`self.ExplosionRadius`) 0.0 (`self.MaxPushForce`))) true true))

(fn `UserConstructionScript`
  (bind _fusetime (`self.FuseTime`))
  (`parent.UserConstructionScript`)
  (`self.SetLifeSpan` (+ _fusetime 0.1))
  (`KismetSystemLibrary.K2_SetTimerDelegate` (`|CreateDelegate` :!event `BANG!`) _fusetime true))