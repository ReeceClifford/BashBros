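; Base weapon projectile Blueprint that moves through a ProjectileMovement component and carries a Mesh.
; Its construction script applies tunable variables to the actor: lifespan, gravity scale, speed and mesh world scale.
; A single Speed value drives both initial and maximum projectile speed.
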(fn `UserConstructionScript`
  (bind _speed (`self.Speed`))
  (bind _projectilemovement (`self.ProjectileMovement`))
  (`self.SetLifeSpan` (`self.TimeToLive`))
  (set `ProjectileMovementComponent.ProjectileGravityScale` (`self.Gravity`) _projectilemovement)
  (set `ProjectileMovementComponent.InitialSpeed` _speed _projectilemovement)
  (set `ProjectileMovementComponent.MaxSpeed` _speed _projectilemovement)
  (`SceneComponent.SetWorldScale3D` (`self.Mesh`) (`self.Scale`)))