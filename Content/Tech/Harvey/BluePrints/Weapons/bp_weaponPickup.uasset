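; Weapon pickup actor that grants a power-up projectile, such as mace, bomb or speed potion, to the main character.
; On BeginPlay, the WeaponToGive enum picks a data table row that sets the mesh and material, then a timeline animates bob and spin.
; On overlap with a Bpc_ThrowingMech owner, it assigns the row's class to that component's ProjectileObtained and destroys itself once the BP_MainCharacter cast succeeds.
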(event `self.ReceiveBeginPlay`
  (bind _staticmesh (`self.StaticMesh`))
  (bind _staticmesh_2 (`self.StaticMesh`))
  (bind _returnvalue (`|GetDataTableRow` (`self.data`) (select `/Game/Tech/Harvey/BluePrints/Weapons/Enum_WeaponList` (`self.WeaponToGive`) :`NewEnumerator1` "Mace" :`NewEnumerator2` "Bomb" :`NewEnumerator3` "Speed" :!type "Name"))
    (:`then`
      (bind (_classforpowerup _mesh _material) (break `/Game/Tech/Harvey/BluePrints/Weapons/Weapons` _returnvalue))
      (`StaticMeshComponent.SetStaticMesh` _staticmesh_2 _mesh)
      (`PrimitiveComponent.SetMaterial` _staticmesh_2 0 _material)
      (bind (_direction _float _spin) (`Timeline|PickUp Do Thing`)
        (:`Update`
          (`SceneComponent.K2_SetRelativeTransform` _staticmesh (`KismetMathLibrary.MakeTransform` (`KismetMathLibrary.VLerp` (0.0 0.0 0.0) (0.0 0.0 40.0) _float) (`KismetMathLibrary.RLerp` (struct) (struct :`Pitch` 340.0 :`Yaw` 360.0 :`Roll` 340.0) _spin) (`SceneComponent.RelativeScale3D` _staticmesh)) false false))))
    (:`RowNotFound`
      (`KismetSystemLibrary.PrintString` "Not In Table"))))

(event `/Game/Tech/Harvey/BluePrints/Weapons/bpi_pickupHelper.PickUpCollected`
  (set `/Game/Tech/Harvey/BluePrints/Weapons/bpc_ThrowingMech.ProjectileObtained` (`.ClassForPowerUp_8_82DE2BD7478BFE50FDE565B20CFA8182` (break `/Game/Tech/Harvey/BluePrints/Weapons/Weapons` (stale `self.ReceiveBeginPlay` _returnvalue))) (`self.ThrowComp Found`)))

(event `self.PickUp Zone.OnComponentBeginOverlap`
  (params (OverlappedComponent :type "PrimitiveComponent Object Reference") (OtherActor :type "Actor Object Reference") (OtherComp :type "PrimitiveComponent Object Reference") (OtherBodyIndex :type Integer) (bFromSweep :type Boolean) (SweepResult :type "HitResult Structure (by ref)"))
  (bind _returnvalue (`self.GetComponentByClass` OtherActor "/Game/Tech/Harvey/BluePrints/Weapons/bpc_ThrowingMech.bpc_ThrowingMech_C"))
  (`/Engine/EditorBlueprintResources/StandardMacros.IsValid` _returnvalue
    (:`Is Valid`
      (set `self.ThrowComp Found` _returnvalue)
      (bind _asbp_main_character (cast `/Game/Tech/Cam/BP_MainCharacter` (`ActorComponent.GetOwner` _returnvalue)))
      (set `self.MainCharacter` _asbp_main_character)
      (`/Game/Tech/Harvey/BluePrints/Weapons/bpi_pickupHelper.PickUpCollected`)
      (`self.K2_DestroyActor`))))

(fn `UserConstructionScript`)