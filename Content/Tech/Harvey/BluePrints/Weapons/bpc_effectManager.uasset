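; Actor component that manages movement and status effects on its owner: stun immunity, a speed boost and a grabbing slowdown.
; On BeginPlay it caches the owner's CharacterMovementComponent and original walk speed.
; ApplyPowerUp routes the selection to functions that set the immunity flag, multiply current speed on a timer, or halve original speed.
; EndEffect restores the original speed, or clears immunity when its Immune input is true.
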(event `self.ReceiveBeginPlay`
  (bind _returnvalue (`self.GetOwner`))
  (if (`KismetSystemLibrary.IsValid` _returnvalue)
    (bind _output_get (set `self.Owner` _returnvalue))
    (bind _returnvalue_2 (`Actor.GetComponentByClass` _output_get "/Script/Engine.CharacterMovementComponent"))
    (`/Engine/EditorBlueprintResources/StandardMacros.IsValid` _returnvalue_2
      (:`Is Valid`
        (set `self.Movement` _returnvalue_2)
        (set `self.Origin Speed` (`CharacterMovementComponent.MaxWalkSpeed` (`self.Movement`)))))))

(event `ApplyPowerUp`
  (params (Selection :type "/Game/Tech/Harvey/BluePrints/Weapons/Enum_PowerUp Enum" :default "NewEnumerator0"))
  (switch `/Game/Tech/Harvey/BluePrints/Weapons/Enum_PowerUp` Selection
    (:`NewEnumerator0`
      (`self.StunImmunity`))
    (:`NewEnumerator1`
      (`self.Speed`))
    (:`NewEnumerator2`
      (`self.Grabbing`))))

(event `Speed Duration`
  (`self.EndEffect` false "NewEnumerator1"))

(fn `EndEffect`
  (params (`Immune?` :type Boolean) (`Power To Stop` :type "/Game/Tech/Harvey/BluePrints/Weapons/Enum_PowerUp Enum" :default "NewEnumerator0"))
  (switch `/Game/Tech/Harvey/BluePrints/Weapons/Enum_PowerUp` `Power To Stop`
    (:`NewEnumerator0`
      (if `Immune?`
        (set `self.ImmuneToStun` false)))
    (:`NewEnumerator1`
      (set `CharacterMovementComponent.MaxWalkSpeed` (`self.Origin Speed`) (`self.Movement`) :!label _label))
    (:`NewEnumerator2`
      (goto _label))))

(fn `Grabbing`
  (set `CharacterMovementComponent.MaxWalkSpeed` (* (`self.Origin Speed`) 0.5) (`self.Movement`)))

(fn `Speed`
  (bind _movement (`self.Movement`))
  (set `CharacterMovementComponent.MaxWalkSpeed` (* (`CharacterMovementComponent.MaxWalkSpeed` _movement) (`self.SpeedBoost`)) _movement)
  (`KismetSystemLibrary.K2_SetTimerDelegate` (`|CreateDelegate` :!event `Speed Duration`) (`self.SpeedBoostDuration`)))

(fn `StunImmunity`
  (set `self.ImmuneToStun` true))