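; bp_EvenField is a pressure-plate button that shows whether something is standing on it and records that in a SteppedOn flag.
; Box overlap begin and end set the flag and call ButtonPressed, which swaps the button material between green and red.
; A Pushing timeline lerps the button down when pressed and reverses to raise it on release, with no filter on the overlapping actor.
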(event `ButtonPressed`
  (params (`On?` :type Boolean))
  (bind _button (`self.Button`))
  (if `On?`
    (`PrimitiveComponent.SetMaterial` _button 0 "/Game/Tech/Harvey/Materials/MI_Solid_GreenDJ.MI_Solid_GreenDJ")
    (bind (_direction _pushing) (`Timeline|Pushing` :!label _label)
      (:`Update`
        (`SceneComponent.K2_SetRelativeLocation` (`self.Button`) (`KismetMathLibrary.VLerp` (0.0 0.0 50.0) (0.0 0.0 35.0) _pushing) false false)))
    (else
      (`PrimitiveComponent.SetMaterial` _button 0 "/Game/Tech/Harvey/Materials/MI_Solid_RedDJ.MI_Solid_RedDJ")
      (goto _label :!via `Reverse`))))

(event `self.Box.OnComponentBeginOverlap`
  (params (OverlappedComponent :type "PrimitiveComponent Object Reference") (OtherActor :type "Actor Object Reference") (OtherComp :type "PrimitiveComponent Object Reference") (OtherBodyIndex :type Integer) (bFromSweep :type Boolean) (SweepResult :type "HitResult Structure (by ref)"))
  (`self.ButtonPressed` true)
  (set `self.SteppedOn?` true))

(event `self.Box.OnComponentEndOverlap`
  (params (OverlappedComponent :type "PrimitiveComponent Object Reference") (OtherActor :type "Actor Object Reference") (OtherComp :type "PrimitiveComponent Object Reference") (OtherBodyIndex :type Integer))
  (`self.ButtonPressed` false)
  (set `self.SteppedOn?` false))

(fn `UserConstructionScript`)