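; Race start line that holds the start until every player button is stepped on.
; On BeginPlay it spawns Bp_EvenField buttons relative to its Wall, choosing placement slots by the game instance's player mode, and initializes a countdown widget with itself.
; A looping half-second timer drives the button check.
; Once all are pressed, it signals that the race is about to begin, then destroys itself after a short delay.
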(event `Create Button`
  (params (Index :type "/Game/Tech/Les/LevelAndModes/E_NumberofPlayers Enum" :default "NewEnumerator5"))
  (for _index (range (select `/Game/Tech/Les/LevelAndModes/E_NumberofPlayers` Index :`NewEnumerator5` 1 :`NewEnumerator1` 1) (+ (select `/Game/Tech/Les/LevelAndModes/E_NumberofPlayers` Index :`NewEnumerator5` 1 :`NewEnumerator1` 2 :`NewEnumerator4` 2 :`NewEnumerator2` 3) 1))
    (`self.Spawn Button` _index)))

(event `self.ReceiveBeginPlay`
  ;[1 1 1] Create Buttons
  (bind _asbp_game_instance (cast `/Game/Tech/Reece/BP_GameInstance` (`GameplayStatics.GetGameInstance`)))
  (`self.Create Button` (`/Game/Tech/Reece/BP_GameInstance.PlayerMode` _asbp_game_instance))
  (`KismetSystemLibrary.K2_SetTimerDelegate` (`|CreateDelegate` :!event `CheckToStart`) 0.5 true)
  (bind _aswbp_countdown (cast `/Game/Tech/Harvey/BluePrints/UI/wbp_Countdown` (`WidgetComponent.GetWidget` (`self.Widget`))))
  (`/Game/Tech/Harvey/BluePrints/UI/wbp_Countdown.Init` _aswbp_countdown self))

(event `CheckToStart`
  (bind _buttons (`self.Buttons`))
  ;[1 1 1] If All Buttons are Pressed
  (for _array_element _buttons
    (if (`/Game/Tech/Harvey/BluePrints/bp_EvenField.SteppedOn?` _array_element)
      (`/Engine/EditorBlueprintResources/StandardMacros.IncrementInt` (`self.ButtonsActivated`))))
  (if (== (`self.ButtonsActivated`) (`KismetArrayLibrary.Array_Length` _buttons))
    (`/Engine/EditorBlueprintResources/StandardMacros.DoOnce` false
      (:`Completed`
        (`self.Race About To Begin`)
        (`KismetSystemLibrary.PrintString` "Start")
        (`KismetSystemLibrary.Delay` 3.0)
        (`self.K2_DestroyActor`)))
    (else
      (set `self.ButtonsActivated` 0))))

(fn `UserConstructionScript`)