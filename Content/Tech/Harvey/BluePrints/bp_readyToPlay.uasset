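; Ready-up zone actor that moves the session to another level once all players stand inside it.
; BeginPlay starts a looping half-second timer, apparently driving ReadyToBegin through a created event.
; ReadyToBegin compares the player controller count with the overlapping BP_MainCharacter count.
; When they match, it runs a servertravel console command with LevelToTravelTo appended directly, with no separator added.
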(event `self.ReceiveBeginPlay`
  (`KismetSystemLibrary.K2_SetTimerDelegate` (`|CreateDelegate` :!event `ReadyToBegin`) 0.5 true))

(event `ReadyToBegin`
  (if (== (`GameplayStatics.GetNumPlayerControllers`) (`KismetArrayLibrary.Array_Length` (`self.GetOverlappingActors` "/Game/Tech/Cam/BP_MainCharacter.BP_MainCharacter_C")))
    (`KismetSystemLibrary.ExecuteConsoleCommand` (`KismetStringLibrary.Concat_StrStr` "servertravel " (`self.Level To Travel To`)) null)))

(fn `UserConstructionScript`)