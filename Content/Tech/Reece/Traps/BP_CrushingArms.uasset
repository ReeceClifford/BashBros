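; Crushing arm trap that drives a Cube component through a looping timeline named MoveDrillArm, set to double speed on BeginPlay.
; Tick calls Play every frame, and the timeline rewinds to zero when finished, so it repeats.
; Each update sets the Cube's world transform from a lerp between StartPoint and EndPoint, though alpha is fixed at zero and BeginPlay assigns both points no value.
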(event `self.ReceiveBeginPlay`
  (set `self.StartPoint` (struct))
  (set `self.EndPoint` (struct))
  (`TimelineComponent.SetPlayRate` (`self.MoveDrillArm`) 2.0))

(event `self.ReceiveTick`
  (params (DeltaSeconds :type "Float (single-precision)"))
  (`Timeline|MoveDrillArm`
    (:`Update`
      (`SceneComponent.K2_SetWorldTransform` (`self.Cube`) (`KismetMathLibrary.TLerp` (`self.StartPoint`) (`self.EndPoint`)) false false))
    (:`Finished`
      (`TimelineComponent.SetNewTime` (`self.MoveDrillArm`) 0.0))))

(fn `UserConstructionScript`)