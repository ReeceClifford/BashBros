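; BP_RadiationField is a trap that randomly stuns the main character while they stay inside its box.
; Entering starts a looping timer that counts exposure and rolls for an odd number in a range that shrinks with exposure.
; A successful roll disables movement for the stun duration, then restores walking and sets a flag that delays further stuns.
; Leaving clears the timer and resets exposure.
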(event `self.Box.OnComponentBeginOverlap`
  (params (OverlappedComponent :type "PrimitiveComponent Object Reference") (OtherActor :type "Actor Object Reference") (OtherComp :type "PrimitiveComponent Object Reference") (OtherBodyIndex :type Integer) (bFromSweep :type Boolean) (SweepResult :type "HitResult Structure (by ref)"))
  ;[1 1 1] Detect Radiation Entered
  (bind _returnvalue (`KismetSystemLibrary.K2_SetTimerDelegate` (delegate `TriggerInZone`) 0.5 true))
  (set `self.Timer` _returnvalue)
  (set `self.beenStunned?` false))

(event `TriggerInZone`
  ;[1 1 1] Apply Radiation Over Time
  (`KismetSystemLibrary.PrintString` "RadiationAdd")
  (bind _result (`/Engine/EditorBlueprintResources/StandardMacros.IncrementInt` (`self.TimeInRadiation`))
    (:`  `
      (bind _output_get (set `self.TimeInRadiation` _result))
      (`KismetSystemLibrary.PrintString` (`KismetStringLibrary.Conv_IntToString` _output_get))
      (if (`self.beenStunned?`)
        (`KismetSystemLibrary.Delay` 5.0)
        (set `self.beenStunned?` false)
        (elif (> (mod (`KismetMathLibrary.RandomIntegerInRange` 1 (- (`self.MaxRadiation`) (`self.TimeInRadiation`))) 2) 0)
          (bind _asbp_main_character (cast `/Game/Tech/Cam/BP_MainCharacter` (stale `self.Box.OnComponentBeginOverlap` OtherActor)))
          (bind _charactermovement (`Character.CharacterMovement` _asbp_main_character))
          (`CharacterMovementComponent.DisableMovement` _charactermovement)
          (`KismetSystemLibrary.Delay` (`self.TimeForStun`))
          (`CharacterMovementComponent.SetMovementMode` _charactermovement "MOVE_Walking" 0)
          (set `self.beenStunned?` true)
          (cast `/Game/Tech/Cam/BP_MainCharacter` (stale `self.Box.OnComponentBeginOverlap` OtherActor)))))))

(event `self.Box.OnComponentEndOverlap`
  (params (OverlappedComponent :type "PrimitiveComponent Object Reference") (OtherActor :type "Actor Object Reference") (OtherComp :type "PrimitiveComponent Object Reference") (OtherBodyIndex :type Integer))
  ;[1 1 1] Reset Count on Exit Trigger
  (`KismetSystemLibrary.K2_ClearAndInvalidateTimerHandle` (`self.Timer`))
  (`KismetSystemLibrary.PrintString` "No Longer In Radiation")
  (set `self.TimeInRadiation` 0))

(fn `UserConstructionScript`)