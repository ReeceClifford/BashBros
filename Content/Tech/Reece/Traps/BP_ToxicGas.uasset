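; Toxic gas trap that respawns the player after too long inside its box volume.
; Overlap start runs a looping one-second timer that increments TimeInGas and, once it reaches HowLongInZone, casts the overlapping actor to BP_MainCharacter and calls RespawnPlayer.
; Overlap end clears the timer and resets the count.
; No incremental damage is applied, and debug prints trace the state.
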(event `self.Box.OnComponentBeginOverlap`
  (params (OverlappedComponent :type "PrimitiveComponent Object Reference") (OtherActor :type "Actor Object Reference") (OtherComp :type "PrimitiveComponent Object Reference") (OtherBodyIndex :type Integer) (bFromSweep :type Boolean) (SweepResult :type "HitResult Structure (by ref)"))
  ;[1 1 1] Detect Gas Entered
  (bind _returnvalue (`KismetSystemLibrary.K2_SetTimerDelegate` (delegate `TriggerInZone`) 1.0 true))
  (set `self.Timer` _returnvalue))

(event `TriggerInZone`
  (bind _timeingas (`self.TimeInGas`))
  ;[1 1 1] Apply Damage over time
  (`KismetSystemLibrary.PrintString` "PlayerInGas")
  (bind _result (`/Engine/EditorBlueprintResources/StandardMacros.IncrementInt` _timeingas)
    (:`  `
      (set `self.TimeInGas` _result)
      (`KismetSystemLibrary.PrintString` (`KismetStringLibrary.Conv_IntToString` _timeingas))
      (if (>= _timeingas (`self.HowLongInZone?`))
        (bind _asbp_main_character (cast `/Game/Tech/Cam/BP_MainCharacter` (stale `self.Box.OnComponentBeginOverlap` OtherActor)))
        (`/Game/Tech/Cam/BP_MainCharacter.RespawnPlayer` _asbp_main_character)))))

(event `self.Box.OnComponentEndOverlap`
  (params (OverlappedComponent :type "PrimitiveComponent Object Reference") (OtherActor :type "Actor Object Reference") (OtherComp :type "PrimitiveComponent Object Reference") (OtherBodyIndex :type Integer))
  ;[1 1 1] Reset Count on Exit Trigger
  (`KismetSystemLibrary.K2_ClearAndInvalidateTimerHandle` (`self.Timer`))
  (`KismetSystemLibrary.PrintString` "No longer In gas")
  (set `self.TimeInGas` 0))

(fn `UserConstructionScript`)